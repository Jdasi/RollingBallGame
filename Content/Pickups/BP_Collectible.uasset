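; BP_Collectible is a base pickup that a BP_RollingBall collects by overlapping it.
; ApplyCollectible is a stub returning false for subclasses to override; on success the pickup plays an optional 2D sound.
; It then either destroys itself or, with a positive RespawnTime, hides its Trigger hierarchy during the delay.
; The overlapping ball is tracked, so a respawned pickup retriggers immediately if one remains inside.
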(event `Retrigger`
  (bind _success (`self.Apply Collectible` (`self.Overlapping Ball`) :!label _label))
  (if _success
    (`self.Common Collect Effects`)
    (if (> (`self.Respawn Time`) 0.0)
      (`self.Set Respawning` true)
      (`KismetSystemLibrary.Delay` (`self.Respawn Time`))
      (`self.Set Respawning` false)
      (if (`KismetSystemLibrary.IsValid` (`self.Overlapping Ball`))
        (`self.Retrigger`))
      (else
        (`self.K2_DestroyActor`)))))

(event `self.ReceiveActorBeginOverlap`
  (params (OtherActor :type "Actor Object Reference"))
  (bind _asbp_rolling_ball (cast `/Game/RollingBall/BP_RollingBall` OtherActor))
  (set `self.Overlapping Ball` _asbp_rolling_ball)
  (if (not (`self.Respawning`))
    (goto _label)))

(event `self.ReceiveActorEndOverlap`
  (params (OtherActor :type "Actor Object Reference"))
  (cast `/Game/RollingBall/BP_RollingBall` OtherActor)
  (set `self.Overlapping Ball` null))

(fn `Apply Collectible`
  (params (`Rolling Ball Character` :type "/Game/RollingBall/BP_RollingBall Object Reference"))
  (returns (Success :type Boolean))
  (return false))

(fn `Common Collect Effects`
  (bind _sound_cue (`self.Sound Cue`))
  (if (`KismetSystemLibrary.IsValid` _sound_cue)
    (`GameplayStatics.PlaySound2D` _sound_cue 1.0 1.0 0.0 null null)))

(fn `Set Respawning`
  (params (Value :type Boolean))
  (`SceneComponent.SetVisibility` (`self.Trigger`) (not Value) true)
  (set `self.Respawning` Value))

(fn `UserConstructionScript`)